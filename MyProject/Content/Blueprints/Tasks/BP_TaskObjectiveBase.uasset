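; Base actor for a task objective that counts interactions toward a required amount and notifies its owning TaskBase when that amount is reached.
; BeginPlay initializes count and image widget components after a short delay; Activate starts a looping flash and makes the sphere block a custom trace channel.
; Interact plays a sound and increments the count, debounced by a resetting DoOnce.
; Completion stops the flash, ignores the trace, then hides the visual or swaps its image.
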(event `self.ReceiveBeginPlay`
  (bind _asw_task_visual (cast `/Game/Blueprints/Tasks/W_TaskVisual` (`WidgetComponent.GetWidget` (`self.WVisual`)) :!pure true))
  (bind _asw_number_count (cast `/Game/Blueprints/Tasks/W_NumberCount` (`WidgetComponent.GetWidget` (`self.WCount`)) :!pure true))
  (`KismetSystemLibrary.Delay` 0.5)
  (`KismetSystemLibrary.DelayUntilNextTick`)
  (set `/Game/Blueprints/Tasks/W_NumberCount.Type` (`/Game/Blueprints/Tasks/BP_TaskBase.TaskType` (`self.TaskBase`)) _asw_number_count)
  (set `/Game/Blueprints/Tasks/W_NumberCount.ObjectiveRef` self _asw_number_count)
  (set `/Game/Blueprints/Tasks/W_TaskVisual.TaskImage` (`self.ObjectiveImage`) _asw_task_visual)
  (`/Game/Blueprints/Tasks/W_TaskVisual.UpdateImage` _asw_task_visual))

(event `StopAnim`
  (bind _asw_task_visual (cast `/Game/Blueprints/Tasks/W_TaskVisual` (`WidgetComponent.GetWidget` (`self.WVisual`)) :!pure true))
  (`UserWidget.StopAnimation` _asw_task_visual (`/Game/Blueprints/Tasks/W_TaskVisual.Flashing` _asw_task_visual))
  (`PrimitiveComponent.SetCollisionResponseToChannel` (`self.Sphere`) "ECC_GameTraceChannel2" "ECR_Ignore"))

(event `ObjectiveReached`
  (bind _currentamount (`self.CurrentAmount`))
  (bind _objectiveimagecomplete (`self.ObjectiveImageComplete`))
  (bind _asw_task_visual (cast `/Game/Blueprints/Tasks/W_TaskVisual` (`WidgetComponent.GetWidget` (`self.WVisual`)) :!pure true))
  (`/Engine/EditorBlueprintResources/StandardMacros.DoOnce` false :!label _label
    (:`Completed`
      (`|ExecutionSequence`
        (:`then_0`
          (if (`self.Active`)
            (`GameplayStatics.PlaySoundAtLocation` (`self.SoundCue`) (`self.K2_GetActorLocation`) (struct) 1.0 1.0 0.0 null null null null)
            (bind _result (`/Engine/EditorBlueprintResources/StandardMacros.IncrementInt` _currentamount)
              (:`  `
                (`KismetSystemLibrary.PrintString` (`KismetStringLibrary.Conv_IntToString` _result))
                (if (== _currentamount (`self.AmountNeeded`))
                  (set `self.Active` false)
                  (`self.StopAnim`)
                  (`/Game/Blueprints/Tasks/BP_TaskBase.CheckForComplete` (`self.TaskBase`))
                  (if (`self.DestroyOnComplete`)
                    (`SceneComponent.SetVisibility` (`self.WVisual`) false false)
                    (`PrimitiveComponent.SetCollisionEnabled` (`self.Sphere`) "NoCollision")
                    (else
                      (`/Engine/EditorBlueprintResources/StandardMacros.IsValid` _objectiveimagecomplete
                        (:`Is Valid`
                          (set `/Game/Blueprints/Tasks/W_TaskVisual.TaskImage` _objectiveimagecomplete _asw_task_visual)
                          (`/Game/Blueprints/Tasks/W_TaskVisual.UpdateImage` _asw_task_visual))))))))))
        (:`then_1`
          (`KismetSystemLibrary.Delay` 0.1)
          (goto _label :!via `Reset`))))))

(event `/Game/Blueprints/Tasks/BPI_Interact.Interact`
  (`self.ObjectiveReached`))

(event `Activate`
  (bind _asw_task_visual (cast `/Game/Blueprints/Tasks/W_TaskVisual` (`WidgetComponent.GetWidget` (`self.WVisual`)) :!pure true))
  (`|ExecutionSequence`
    (:`then_0`
      (`/Engine/EditorBlueprintResources/StandardMacros.DoOnce` false
        (:`Completed`
          (set `self.Active` true))))
    (:`then_1`
      (if (not (== (`self.AmountNeeded`) (`self.CurrentAmount`)))
        (`UserWidget.PlayAnimation` _asw_task_visual (`/Game/Blueprints/Tasks/W_TaskVisual.Flashing` _asw_task_visual) 0.0 0 "Forward" 1.0 false)
        (`PrimitiveComponent.SetCollisionResponseToChannel` (`self.Sphere`) "ECC_GameTraceChannel2" "ECR_Block")))))

(fn `UserConstructionScript`)