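; BP_Projectile is a task projectile actor that displays an image and completes a task objective when it touches one.
; On BeginPlay it passes its Image to the W_TaskVisual in its widget component and refreshes it.
; When its Sphere overlaps a BP_TaskObjectiveBase, a DoOnce gate calls ObjectiveReached on that objective, then the projectile destroys itself.
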(event `self.ReceiveBeginPlay`
  (bind _asw_task_visual (cast `/Game/Blueprints/Tasks/W_TaskVisual` (`WidgetComponent.GetWidget` (`self.Widget`)) :!pure true))
  (set `/Game/Blueprints/Tasks/W_TaskVisual.TaskImage` (`self.Image`) _asw_task_visual)
  (`/Game/Blueprints/Tasks/W_TaskVisual.UpdateImage` _asw_task_visual))

(event `self.Sphere.OnComponentBeginOverlap`
  (params (OverlappedComponent :type "PrimitiveComponent Object Reference") (OtherActor :type "Actor Object Reference") (OtherComp :type "PrimitiveComponent Object Reference") (OtherBodyIndex :type Integer) (bFromSweep :type Boolean) (SweepResult :type "HitResult Structure (by ref)"))
  (bind _asbp_task_objective_base (cast `/Game/Blueprints/Tasks/BP_TaskObjectiveBase` OtherActor))
  (`/Engine/EditorBlueprintResources/StandardMacros.DoOnce` false
    (:`Completed`
      (`/Game/Blueprints/Tasks/BP_TaskObjectiveBase.ObjectiveReached` _asbp_task_objective_base)
      (`self.K2_DestroyActor`))))

(fn `UserConstructionScript`)