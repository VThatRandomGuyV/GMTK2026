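; BP_TaskFuse is an interactable fuse task that ends the current day once it has been activated.
; Activate sets the Active flag and loops the Flashing animation on its W_TaskVisual widget.
; Interact calls the parent, then, if active, runs once to increment CurrentDay on BP_GameInstance, print it, and open Lvl_MainHome after a short delay.
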(event `Activate`
  (bind _asw_task_visual (cast `/Game/Blueprints/Tasks/W_TaskVisual` (`WidgetComponent.GetWidget` (`self.Widget`)) :!pure true))
  (set `self.Active` true)
  (`UserWidget.PlayAnimation` _asw_task_visual (`/Game/Blueprints/Tasks/W_TaskVisual.Flashing` _asw_task_visual) 0.0 0 "Forward" 1.0 false))

(event `/Game/Blueprints/Tasks/BPI_Interact.Interact`
  (`parent.Interact`)
  (if (`self.Active`)
    (`/Engine/EditorBlueprintResources/StandardMacros.DoOnce` false
      (:`Completed`
        (bind _result (`/Engine/EditorBlueprintResources/StandardMacros.IncrementInt` (`/Game/Blueprints/Managers/BP_GameInstance.CurrentDay` (cast `/Game/Blueprints/Managers/BP_GameInstance` (`GameplayStatics.GetGameInstance`) :!pure true)))
          (:`  `
            (`KismetSystemLibrary.PrintString` (`KismetStringLibrary.Conv_IntToString` _result))
            (`KismetSystemLibrary.Delay` 0.3)
            (`GameplayStatics.OpenLevelBySoftObjectPtr` "/Game/Levels/Lvl_MainHome.Lvl_MainHome")))))))

(fn `UserConstructionScript`
  (`parent.UserConstructionScript`))