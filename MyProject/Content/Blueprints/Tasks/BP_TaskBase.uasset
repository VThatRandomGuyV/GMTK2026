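; Base task actor with a widget icon that flashes while active and, on interaction, hands the player a task and activates its attached objectives.
; Objectives receive a back-reference at BeginPlay, letting CheckForComplete finish the task once none remain active.
; Completion activates the first BP_TaskFuse found, resets the player's task, then either destroys the actor or shows a completion image and disables interaction.
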(event `self.ReceiveBeginPlay`
  (bind _asw_task_visual (cast `/Game/Blueprints/Tasks/W_TaskVisual` (`WidgetComponent.GetWidget` (`self.Widget`)) :!pure true))
  (for _array_element (`self.AttachedObjectives`)
    (set `/Game/Blueprints/Tasks/BP_TaskObjectiveBase.TaskBase` self _array_element))
  (set `/Game/Blueprints/Tasks/W_TaskVisual.TaskImage` (`self.TaskImage`) _asw_task_visual)
  (`/Game/Blueprints/Tasks/W_TaskVisual.UpdateImage` _asw_task_visual)
  (if (`self.Active`)
    (`KismetSystemLibrary.DelayUntilNextTick`)
    (`UserWidget.PlayAnimation` _asw_task_visual (`/Game/Blueprints/Tasks/W_TaskVisual.Flashing` _asw_task_visual) 0.0 0 "Forward" 1.0 false :!label _label)
    (`KismetSystemLibrary.PrintString` "Hello")))

(event `PlayAnim`
  (goto _label))

(event `/Game/Blueprints/Tasks/BPI_Interact.Interact`
  (bind _widget (`self.Widget`))
  (bind _asw_task_visual (cast `/Game/Blueprints/Tasks/W_TaskVisual` (`WidgetComponent.GetWidget` _widget) :!pure true))
  (if (`self.Active`)
    (`GameplayStatics.PlaySoundAtLocation` (`self.SoundCue`) (`self.K2_GetActorLocation`) (struct) 1.0 1.0 0.0 null null null null)
    (`|ExecutionSequence`
      (:`then_0`
        (for _array_element (`self.AttachedObjectives`)
          (`/Game/Blueprints/Tasks/BP_TaskObjectiveBase.Activate` _array_element)))
      (:`then_1`
        (`/Game/Blueprints/BP_PlayerCharacter.ReloadTask` (cast `/Game/Blueprints/BP_PlayerCharacter` (`GameplayStatics.GetPlayerCharacter` 0) :!pure true) (`self.TaskType`) (`self.Amount`) (`self.EquipImage`))
        (`UserWidget.StopAnimation` _asw_task_visual (`/Game/Blueprints/Tasks/W_TaskVisual.Flashing` _asw_task_visual))
        (if (or (`|EnumEquality` (`self.TaskType`) "NewEnumerator2") (`self.HideOnPickup`))
          (`SceneComponent.SetVisibility` _widget false false)
          (`PrimitiveComponent.SetCollisionResponseToChannel` (`self.InteractCollision`) "ECC_GameTraceChannel2" "ECR_Ignore"))))))

(fn `CheckForComplete`
  (bind _asw_task_visual (cast `/Game/Blueprints/Tasks/W_TaskVisual` (`WidgetComponent.GetWidget` (`self.Widget`)) :!pure true))
  (for _array_element (`self.AttachedObjectives`)
    (if (`/Game/Blueprints/Tasks/BP_TaskObjectiveBase.Active` _array_element)
      (return)))
  (`|ExecutionSequence`
    (:`then_0`
      (bind _returnvalue (`GameplayStatics.GetActorOfClass` "/Game/Blueprints/Tasks/BP_TaskFuse.BP_TaskFuse_C"))
      (`/Engine/EditorBlueprintResources/StandardMacros.IsValid` _returnvalue
        (:`Is Valid`
          (`/Game/Blueprints/Tasks/BP_TaskFuse.Activate` _returnvalue))))
    (:`then_1`
      (`/Game/Blueprints/BP_PlayerCharacter.ReloadTask` (cast `/Game/Blueprints/BP_PlayerCharacter` (`GameplayStatics.GetPlayerCharacter` 0) :!pure true) "NewEnumerator0" 0.0 null)
      (if (`self.DeleteOnComplete`)
        (`self.K2_DestroyActor`)
        (else
          (set `/Game/Blueprints/Tasks/W_TaskVisual.TaskImage` (`self.TaskCompleteImage`) _asw_task_visual)
          (`/Game/Blueprints/Tasks/W_TaskVisual.UpdateImage` _asw_task_visual)
          (`PrimitiveComponent.SetCollisionResponseToChannel` (`self.InteractCollision`) "ECC_GameTraceChannel2" "ECR_Ignore")
          (`UserWidget.StopAnimation` _asw_task_visual (`/Game/Blueprints/Tasks/W_TaskVisual.Flashing` _asw_task_visual))
          (`SceneComponent.SetVisibility` (`self.Widget`) true false))))))

(fn `UserConstructionScript`)