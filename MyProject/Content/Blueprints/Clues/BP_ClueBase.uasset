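; BP_ClueBase is an interactable clue actor configured by a row in DT_Clues.
; On BeginPlay it destroys itself if the game instance already lists that clue as found, otherwise showing either a decal or a widget image.
; When active, its first interaction records the clue in both game instance and game mode, opens a W_CluePopup, then stops responding on its interaction trace channel.
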(event `self.ReceiveBeginPlay`
  (bind (_clueinfo_datatable _clueinfo_rowname) (break `DataTableRowHandle` (`self.ClueInfo`)))
  (bind _asw_task_visual (cast `/Game/Blueprints/Tasks/W_TaskVisual` (`WidgetComponent.GetWidget` (`self.Widget`)) :!pure true))
  (bind _returnvalue (`|GetDataTableRow` "/Game/Blueprints/Clues/DT_Clues.DT_Clues" _clueinfo_rowname)
    (:`then`
      (if (`KismetArrayLibrary.Array_Contains` (`/Game/Blueprints/Managers/BP_GameInstance.CluesFound` (cast `/Game/Blueprints/Managers/BP_GameInstance` (`GameplayStatics.GetGameInstance`) :!pure true)) _returnvalue)
        (`self.K2_DestroyActor`)
        (else
          (bind (_ispopup _isdecal _decalmat _image) (break `/Game/Blueprints/Clues/Str_ClueInfo` _returnvalue))
          (if _isdecal
            (`DecalComponent.SetDecalMaterial` (`self.Decal`) _decalmat)
            (`SceneComponent.SetVisibility` (`self.Widget`) false false)
            (else
              (set `/Game/Blueprints/Tasks/W_TaskVisual.TaskImage` _image _asw_task_visual)
              (`/Game/Blueprints/Tasks/W_TaskVisual.UpdateImage` _asw_task_visual)
              (`SceneComponent.SetVisibility` (`self.Decal`) false false))))))))

(event `self.Interact`
  (bind (_clueinfo_datatable _clueinfo_rowname) (break `DataTableRowHandle` (`self.ClueInfo`)))
  (if (`self.Active`)
    (`/Engine/EditorBlueprintResources/StandardMacros.DoOnce` false
      (:`Completed`
        (`|ExecutionSequence`
          (:`then_0`
            (set `self.Active` false)
            (bind _returnvalue (`|GetDataTableRow` "/Game/Blueprints/Clues/DT_Clues.DT_Clues" _clueinfo_rowname)
              (:`then`
                (`KismetArrayLibrary.Array_AddUnique` (`/Game/Blueprints/Managers/BP_GameInstance.CluesFound` (cast `/Game/Blueprints/Managers/BP_GameInstance` (`GameplayStatics.GetGameInstance`) :!pure true)) _returnvalue)
                (`KismetArrayLibrary.Array_AddUnique` (`/Game/FirstPerson/Blueprints/BP_FirstPersonGameMode.FoundClues` (cast `/Game/FirstPerson/Blueprints/BP_FirstPersonGameMode` (`GameplayStatics.GetGameMode`) :!pure true)) _returnvalue)
                (bind _returnvalue_2 (`|CreateWidget` "/Game/Blueprints/Clues/W_CluePopup.W_CluePopup_C" null _returnvalue))
                (`UserWidget.AddToViewport` _returnvalue_2 0))))
          (:`then_1`
            (`PrimitiveComponent.SetCollisionResponseToChannel` (`self.InteractCollision`) "ECC_GameTraceChannel2" "ECR_Ignore")))))))

(fn `UserConstructionScript`)