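; Modular sword actor that assembles a blade, crossguard, pommel and grip from data tables in its Construction Script.
; Each index selects a table row, falling back to row "0", with blade tables chosen by type and broken variant.
; Metal parts share one dynamic material instance, while grip leather gets parameter-driven variant and colours.
; Crossguard and pommel socket onto the grip, blade onto the crossguard; Random rerolls indexes and rebuilds.
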(fn `Create Sword by Indexes`
  (params (`Blade Index` :type Integer) (`Crossguard Index` :type Integer) (`Pommel Index` :type Integer) (`Grip Index` :type Integer) (`Grip Material Index` :type Integer))
  (locals (`Dynamic Material Instance - Metal` :type "MaterialInstanceDynamic Object Reference"))
  (`|ExecutionSequence`
    (:`then_0`
      (bind _returnvalue (`self.Get DataTable - Blades`))
      (bind _dynamic_material_instance (`self.Set Mesh and Material Instance` _returnvalue (`KismetStringLibrary.Conv_StringToName` (`KismetStringLibrary.Conv_IntToString` `Blade Index`)) (`self.Blade`) 0 (`local.Dynamic Material Instance - Metal`) (`self.Metal Material Index`) true))
      (set `local.Dynamic Material Instance - Metal` _dynamic_material_instance))
    (:`then_1`
      (`self.Set Mesh and Material Instance` (`self.Crossguards`) (`KismetStringLibrary.Conv_StringToName` (`KismetStringLibrary.Conv_IntToString` `Crossguard Index`)) (`self.Crossguard`) 0 (`local.Dynamic Material Instance - Metal`) (`self.Metal Material Index`) true))
    (:`then_2`
      (`self.Set Mesh and Material Instance` (`self.Pommels`) (`KismetStringLibrary.Conv_StringToName` (`KismetStringLibrary.Conv_IntToString` `Pommel Index`)) (`self.Pommel`) 0 (`local.Dynamic Material Instance - Metal`) (`self.Metal Material Index`) true))
    (:`then_3`
      (bind _dynamic_material_instance_2 (`self.Set Mesh and Material Instance` (`self.Grips`) (`KismetStringLibrary.Conv_StringToName` (`KismetStringLibrary.Conv_IntToString` `Grip Index`)) (`self.Grip`)))
      (`MaterialInstanceDynamic.SetScalarParameterValue` _dynamic_material_instance_2 (`self.Material Param - Index`) (select `int` `Grip Material Index` :`0` 1.0 :`1` 0.0 :`2` 0.2 :`3` 0.4 :`4` 0.6 :`5` 0.8))
      (`MaterialInstanceDynamic.SetVectorParameterValue` _dynamic_material_instance_2 (`self.Material Param - Leather A`) (`self.Leather Colour A`))
      (`MaterialInstanceDynamic.SetVectorParameterValue` _dynamic_material_instance_2 (`self.Material Param - Leather B`) (`self.Leather Colour B`)))
    (:`then_4`
      (`self.Set Mesh and Material Instance` (`self.Grips`) (`KismetStringLibrary.Conv_StringToName` (`KismetStringLibrary.Conv_IntToString` `Grip Index`)) (`self.Grip`) 1 (`local.Dynamic Material Instance - Metal`) (`self.Metal Material Index`) true))
    (:`then_5`
      (`self.Set Components To Sockets`))))

(fn `Get DataTable - Blades`
  (returns (ReturnValue :type "DataTable Object Reference"))
  (bind _sword_type (`self.Sword Type`))
  (return (select `byte` (`self.Blade Type`) :`0` (select `byte` _sword_type :`0` (`self.Longblades`) :`1` (`self.Shortblades`)) :`1` (select `byte` _sword_type :`0` (`self.Longblades_Broken`) :`1` (`self.Shortblades_Broken`)))))

(fn `Get Random Index`
  (params (Table :type "DataTable Object Reference"))
  (returns (ReturnValue :type Integer))
  (locals (`Random Index` :type Integer :default 0))
  (set `local.Random Index` 0)
  (bind _outrownames (`DataTableFunctionLibrary.GetDataTableRowNames` Table))
  (for _ _outrownames
    (`/Engine/EditorBlueprintResources/StandardMacros.IncrementInt` (`local.Random Index`)))
  (return (`KismetMathLibrary.RandomIntegerInRange` 0 (`local.Random Index`))))

(fn `Initialise Sword`
  (params (`Is Random?` :type Boolean) (`Blade Index` :type Integer) (`Crossguard Index` :type Integer) (`Pommel Index` :type Integer) (`Grip Index` :type Integer) (`Grip Material Index` :type Integer))
  (if `Is Random?`
    (`self.Random`)
    (else
      (`|ExecutionSequence`
        (:`then_0`
          (set `self.Blade Index` `Blade Index`))
        (:`then_1`
          (set `self.Crossguard Index` `Crossguard Index`))
        (:`then_2`
          (set `self.Pommel Index` `Pommel Index`))
        (:`then_3`
          (set `self.Grip Index` `Grip Index`))
        (:`then_4`
          (set `self.Grip Material Index` `Grip Material Index`))))))

(fn `Random`
  (locals (`Random Index` :type Integer :default 0))
  (`|ExecutionSequence`
    (:`then_0`
      (bind _returnvalue (`self.Get DataTable - Blades`))
      (bind _returnvalue_2 (`self.Get Random Index` _returnvalue))
      (set `self.Blade Index` _returnvalue_2))
    (:`then_1`
      (bind _returnvalue_3 (`self.Get Random Index` (`self.Pommels`)))
      (set `self.Pommel Index` _returnvalue_3))
    (:`then_2`
      (bind _returnvalue_4 (`self.Get Random Index` (`self.Crossguards`)))
      (set `self.Crossguard Index` _returnvalue_4))
    (:`then_3`
      (bind _returnvalue_5 (`self.Get Random Index` (`self.Grips`)))
      (set `self.Grip Index` _returnvalue_5))
    (:`then_4`
      (set `self.Grip Material Index` (`KismetMathLibrary.RandomIntegerInRange` 1 5)))
    (:`then_5`
      (`self.Create Sword by Indexes` (`self.Blade Index`) (`self.Crossguard Index`) (`self.Pommel Index`) (`self.Grip Index`) (`self.Grip Material Index`)))))

(fn `Set Components To Sockets`
  (`SceneComponent.K2_DetachFromComponent` (`self.Crossguard`) "KeepRelative" "KeepRelative" "KeepRelative" true)
  (`SceneComponent.K2_AttachToComponent` (`self.Crossguard`) (`self.Grip`) (`self.Crossguard Socket Name`) "KeepRelative" "KeepRelative" "KeepRelative" true)
  (`SceneComponent.K2_DetachFromComponent` (`self.Pommel`) "KeepRelative" "KeepRelative" "KeepRelative" true)
  (`SceneComponent.K2_AttachToComponent` (`self.Pommel`) (`self.Grip`) (`self.Pommel Socket Name`) "KeepRelative" "KeepRelative" "KeepRelative" true)
  (`SceneComponent.K2_DetachFromComponent` (`self.Blade`) "KeepRelative" "KeepRelative" "KeepRelative" true)
  (`SceneComponent.K2_AttachToComponent` (`self.Blade`) (`self.Crossguard`) (`self.Blade Socket Name`) "KeepRelative" "KeepRelative" "KeepRelative" true))

(fn `Set Mesh and Material Instance`
  (params (`Data Table` :type "DataTable Object Reference") (`Row Name` :type Name) (`Component Ref` :type "StaticMeshComponent Object Reference") (`Material Index` :type Integer) (`Dynamic Material Instance - Input` :type "MaterialInstanceDynamic Object Reference") (`Metal Material Index` :type Integer) (`Use Metal` :type Boolean))
  (returns (`Dynamic Material Instance` :type "MaterialInstanceDynamic Object Reference"))
  (locals (Table_Row :type "/Game/UnrealBucket/Library/Weapon/ModularSwordsPack/Helpers/Structure/ST_SwordComponents Structure"))
  (bind _returnvalue (`KismetSystemLibrary.IsValid` `Dynamic Material Instance - Input`))
  (bind (_staticmesh _listofmaterialsindex0 _listofmaterialsindex1) (break `/Game/UnrealBucket/Library/Weapon/ModularSwordsPack/Helpers/Structure/ST_SwordComponents` (`local.Table_Row`)))
  (bind _returnvalue_2 (`|GetDataTableRow` `Data Table` `Row Name`)
    (:`then`
      (set `local.Table_Row` _returnvalue_2))
    (:`RowNotFound`
      (bind _returnvalue_3 (`|GetDataTableRow` `Data Table` "0")
        (:`then`
          (set `local.Table_Row` _returnvalue_3)))))
  (`StaticMeshComponent.SetStaticMesh` `Component Ref` _staticmesh)
  (if (not _returnvalue)
    (bind _returnvalue_4 (`KismetMaterialLibrary.CreateDynamicMaterialInstance` (select `bool` `Use Metal` :`false` (`|GetArrayItem` _listofmaterialsindex0) :`true` (`|GetArrayItem` _listofmaterialsindex1 `Metal Material Index`) :!type "MaterialInterface Object Reference"))))
  (`PrimitiveComponent.SetMaterial` `Component Ref` `Material Index` (select `bool` _returnvalue :`false` _returnvalue_4 :`true` `Dynamic Material Instance - Input` :!type "MaterialInterface Object Reference"))
  (return _returnvalue_4))

(fn `UserConstructionScript`
  (`self.Create Sword by Indexes` (`self.Blade Index`) (`self.Crossguard Index`) (`self.Pommel Index`) (`self.Grip Index`) (`self.Grip Material Index`)))